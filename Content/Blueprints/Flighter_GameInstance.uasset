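; Game instance for Flighter that holds lives and collected capsule count and decides when the game is won or lost.
; On player death it spends a life and reloads the current level by name, or opens the bad-ending menu when none remain.
; Each collected capsule increments the count, and reaching six opens the good-ending menu.
; Neither counter is reset here, so both carry across level reloads.
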(event Custom|OnPlayerDies
  (if (<= (Variables|Default|GetLives) 0)
    (Game|OpenLevel(byObjectReference) "/Game/Maps/GameMenu_Bad.GameMenu_Bad")
    (else
      (Math|Integer|DecrementInt (Variables|Default|GetLives)
        (:%20%20
          (CallFunction|RestartLevel))))))

(event Custom|OnCapsuleCollected
  (bind _result (Math|Integer|IncrementInt (Variables|Default|GetCapsulesCollected))
    (:%20%20
      (Variables|Default|SetCapsulesCollected _result)
      (if (>= (Variables|Default|GetCapsulesCollected) 6)
        (Game|OpenLevel(byObjectReference) "/Game/Maps/GameMenu_Good.GameMenu_Good")))))

(event EventInit)

(fn RestartLevel
  (bind _returnvalue (Game|GetCurrentLevelName true))
  (Game|OpenLevel(byName) (Utilities|String|StringToName _returnvalue)))